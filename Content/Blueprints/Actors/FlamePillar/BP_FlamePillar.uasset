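; Flame pillar actor that continuously flickers its FlameLight to imitate a burning fire.
; From BeginPlay it randomly plays one of two timelines, each supplying a FlameIntensity curve that scales BaseIntensity on the light every update.
; When a timeline finishes it picks again at random, forming an endless loop of varied flicker without using Tick.
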(event `self.ReceiveBeginPlay`
  (`self.ChooseFlame`))

(event `ChooseFlame`
  (switch `int` (`KismetMathLibrary.RandomIntegerInRange` 0 1)
    (:`Default`
      (`self.StartFlame2` :!label _label))
    (:`0`
      (`self.StartFlame1`))
    (:`1`
      (goto _label))))

(event `StartFlame1`
  (bind (_direction _flameintensity) (`Timeline|Timeline_1` :!via `PlayFromStart`)
    (:`Update`
      (`self.UpdateFlameIntensity` _flameintensity))
    (:`Finished`
      (`self.ChooseFlame`))))

(event `StartFlame2`
  (bind (_direction _flameintensity) (`Timeline|Timeline_2` :!via `PlayFromStart`)
    (:`Update`
      (`self.UpdateFlameIntensity` _flameintensity))
    (:`Finished`
      (`self.ChooseFlame`))))

(fn `UpdateFlameIntensity`
  (params (ScaleIntensityValue :type "Float (double-precision)"))
  (`LightComponent.SetIntensity` (`self.FlameLight`) (* ScaleIntensityValue (`self.BaseIntensity`))))

(fn `UserConstructionScript`)